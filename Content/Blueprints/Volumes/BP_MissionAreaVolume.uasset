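; BP_MissionAreaVolume is a mission boundary volume that punishes a BP_Marine for leaving the play area.
; On overlap end it flags the marine as OutsideMissionArea and starts a Kill_Player timer lasting SecondsBeforePlayerDeath.
; Re-entering clears the flag and cancels the timer.
; If the timer fires, Kill_Player applies 100 damage to player character 0, regardless of which marine left.
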(event EventBeginPlay)

(event Collision|EventActorBeginOverlap
  (params (OtherActor :type Actor%20Object%20Reference))
  ;[1 1 1] 玩家位于任务区内
  (bind _asbp_marine (Utilities|Casting|CastToBP_Marine OtherActor))
  (Variables|/Game/Blueprints/Pawns/BP_Marine.BP_Marine_C|SetOutside_MissionArea _asbp_marine false)
  (Utilities|Time|ClearTimerbyFunctionName 0 "Kill_Player"))

(event EventTick
  (params (DeltaSeconds :type Float%20%28single-precision%29)))

(event Collision|EventActorEndOverlap
  (params (OtherActor :type Actor%20Object%20Reference))
  ;[1 1 1] 玩家位于任务区外
  (bind _asbp_marine (Utilities|Casting|CastToBP_Marine OtherActor))
  (Variables|/Game/Blueprints/Pawns/BP_Marine.BP_Marine_C|SetOutside_MissionArea _asbp_marine true)
  (Utilities|Time|SetTimerbyFunctionName 0 "Kill_Player" (Variables|Default|GetSeconds_BeforePlayerDeath)))

(fn ConstructionScript)

(fn KillPlayer
  (Game|Damage|ApplyDamage (Game|GetPlayerCharacter 0) 1e+02 0 0))