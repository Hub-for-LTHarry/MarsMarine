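; Player Marine for what appears to be a twin-stick shooter, with world-axis movement, health, death, kill count and HUD.
; Tick sets control-rotation yaw from thumbstick direction or smoothed mouse velocity, each with a deadzone, switching on the last key's device.
; Firing runs looping sound and muzzle effects while a timer repeats line traces from the muzzle socket along control rotation, applying damage and impact particles.
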(event EventBeginPlay
  (bind _returnvalue (UserInterface|CreateWidget "/Game/UI/W_PlayerHUD.W_PlayerHUD_C" 0 self))
  (UserInterface|Viewport|AddtoViewport _returnvalue 0))

(event Collision|EventActorBeginOverlap
  (params (OtherActor :type Actor%20Object%20Reference)))

(event EventTick
  (params (DeltaSeconds :type Float%20%28single-precision%29))
  (if (CallFunction|IsAlive)
    (CallFunction|UpdatePlayerAim)))

(event Game|Damage|EventAnyDamage
  (params (Damage :type Float%20%28single-precision%29) (DamageType :type Damage%20Type%20Object%20Reference) (InstigatedBy :type Controller%20Object%20Reference) (DamageCauser :type Actor%20Object%20Reference))
  (if (CallFunction|IsAlive)
    (bind _health (CallFunction|DecreaseHealth Damage))
    (if (== _health 0.0)
      (Variables|Default|SetDead true)
      (CallFunction|StopFiring))))

(event Input|ActionEvents|InputActionFire_Weapon
  (params (Key :type Key%20Structure :default "None"))
  (:Pressed
    (CallFunction|StartFiring)
    (CallFunction|WeaponTrace))
  (:Released
    (CallFunction|StopFiring)))

(event Input|AxisEvents|InputAxisM_Forward
  (params (AxisValue :type Float%20%28single-precision%29))
  (if (CallFunction|IsAlive)
    (Pawn|Input|AddMovementInput "1.000000, 0, 0" AxisValue false)))

(event Input|AxisEvents|InputAxisM_LR
  (params (AxisValue :type Float%20%28single-precision%29))
  (if (CallFunction|IsAlive)
    (Pawn|Input|AddMovementInput "0.000000,1.000000, 0" AxisValue false)))

(event Input|KeyboardEvents|AnyKey
  (params (Key :type Key%20Structure :default "None"))
  (:Pressed
    (Variables|ThumbstickInput|SetGamepad_Active (Class|KismetInputLibrary|KeyIsGamepadKey Key))))

(fn ConstructionScript)

(fn UpdatePlayerAim
  (if (Variables|ThumbstickInput|GetGamepad_Active)
    (ThumbstickInput|UpdateThumbstickAiming)
    (else
      (鼠标输入|UpdateMouseAim))))

(fn IsThumbstickAboveDeadzone
  (return (> (Math|Vector2D|Vector2DLength (Math|Vector2D|MakeVector2D (Input|AxisValues|GetThumbstick_AimUp) (Input|AxisValues|GetThumbstick_AimRight))) (Variables|ThumbstickInput|GetThumbstick_Deadzone))))

(fn GetMouseVelocity
  (bind _returnvalue (Game|GetPlayerController 0))
  (bind (_deltax _deltay) (Class|PlayerController|GetInputMouseDelta _returnvalue))
  (return (/ (Math|Vector2D|MakeVector2D _deltax _deltay) (Utilities|Time|GetWorldDeltaSeconds))))

(fn IsMouseAboveDeadzone
  (return (> (Math|Vector2D|Vector2DLength (鼠标输入|GetMouseVelocity)) (Variables|鼠标输入|GetMouse_Deadzone))))

(fn UpdateMouseAim
  (if (鼠标输入|IsMouseAboveDeadzone)
    (Pawn|SetControlRotation (Game|GetPlayerController 0) (鼠标输入|GetMouseAimDirection))))

(fn UpdateThumbstickAiming
  (if (ThumbstickInput|IsThumbstickAboveDeadzone)
    (Pawn|SetControlRotation (Game|GetPlayerController 0) (ThumbstickInput|GetThumbstickAimDirection))))

(fn GetThumbstickAimDirection
  (return (Math|Rotator|MakeRotator 0.0 0.0 (Class|KismetMathLibrary|DegAtan2 (Input|AxisValues|GetThumbstick_AimUp) (Input|AxisValues|GetThumbstick_AimRight)))))

(fn GetMouseAimDirection
  (bind _returnvalue (鼠标输入|GetMouseVelocity))
  (return (Math|Interpolation|RInterpTo (Pawn|GetControlRotation (Game|GetPlayerController 0) :!class /Script/Engine.Controller) (Math|Rotator|MakeRotator 0.0 0.0 (Class|KismetMathLibrary|DegAtan2 (.x _returnvalue) (.y _returnvalue))) (Utilities|Time|GetWorldDeltaSeconds) (Variables|鼠标输入|GetMouse_Smoothing_Strength))))

(fn StartFiring
  (if (CallFunction|IsAlive)
    (Components|Activation|Activate (Variables|Default|GetP_AssaultRifle_MF) false)
    (bind _returnvalue (Audio|SpawnSound2D "/Game/Sounds/Weapon_AssaultRifle/Stereo/RifleFiringLoop_Cue.RifleFiringLoop_Cue" 1.0 1.0 0.0 0 false false))
    (Variables|Default|SetWeapon_Firing_Sound _returnvalue)
    (CallFunction|WeaponTrace)
    (Utilities|Time|SetTimerbyFunctionName 0 "Weapon_Trace" (Variables|Default|GetWeapon_FireRate) true)))

(fn StopFiring
  (Components|Activation|Deactivate (Variables|Default|GetP_AssaultRifle_MF))
  (Audio|Components|Audio|Stop (Variables|Default|GetWeapon_Firing_Sound))
  (Utilities|Time|ClearTimerbyFunctionName 0 "Weapon_Trace")
  (if (CallFunction|IsAlive)
    (Audio|SpawnSound2D "/Game/Sounds/Weapon_AssaultRifle/Stereo/RifleFireEnd_Cue.RifleFireEnd_Cue" 1.0 1.0 0.0 0 false false)))

(fn DecreaseHealth
  (params (Damage_Amount :type Float%20%28single-precision%29))
  (bind _output_get (Variables|Player_Properties|SetHealth (- (Variables|Player_Properties|GetHealth) Damage_Amount)))
  (return _output_get))

(fn IsAlive
  (return (not (Variables|Default|GetDead))))

(fn WeaponTrace
  (bind _outhit (Collision|LineTraceByChannel (CallFunction|GetWeaponTraceStartLocation) (CallFunction|GetWeaponTraceEndLocation) "TraceTypeQuery1" false 0 "None"))
  (if (.bBlockingHit (Collision|BreakHitResult _outhit))
    (Game|Damage|ApplyDamage (.HitActor (Collision|BreakHitResult _outhit)) (Variables|Default|GetDamage_PerShot) 0 0)
    (CallFunction|SpawnImpactHit (.Location (Collision|BreakHitResult _outhit)))))

(fn GetWeaponTraceStartLocation
  (return (Transformation|GetSocketLocation (Variables|Default|GetRifle) "MuzzleFlash")))

(fn GetWeaponTraceEndLocation
  (return (+ (CallFunction|GetWeaponTraceStartLocation) (* (Math|Vector|GetForwardVector (Pawn|GetControlRotation :!class /Script/Engine.Pawn)) (Variables|Default|GetWeapon_Range)))))

(fn IncreaseKills
  (Math|Integer|IncrementInt (Variables|PlayerProperties|GetKills)))

(fn SpawnImpactHit
  (params (Hit%20Location :type Vector))
  (Effects|SpawnEmitteratLocation "/Game/Effects/Weapons/Impacts/P_AssaultRifle_IH.P_AssaultRifle_IH" Hit%20Location))

(fn AddHealth
  (params (Health_ToAdd :type Float%20%28single-precision%29))
  (Variables|Player_Properties|SetHealth (Math|Float|Clamp(Float) (+ (Variables|Player_Properties|GetHealth) Health_ToAdd) 0.0 1e+02)))

(fn IsHealthFull
  (return (== (Variables|Player_Properties|GetHealth) 1e+02)))